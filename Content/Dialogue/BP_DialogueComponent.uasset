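; Actor component that runs data-table-driven dialogue, showing lines in WB_Dialogue with the mouse cursor enabled.
; Each Interaction opens the widget or advances it, as every row supplies the next table, row and end flag.
; Open-ended choices become WB_Option buttons only when the widget is created; OptionSelected clears them and jumps to the chosen row.
; LeaveDialogue, or Interaction after an end-flagged line, removes the widget and restores game-only input.
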(event Custom|OptionSelected
  (params (DataTable :type Data%20Table%20Object%20Reference) (RowName :type Name))
  ;[0.9635 0.5475 0.1907 0.5] Upon an option being selected update the widget to go to the correct data table row/update the tags
  (bind _returnvalue (Utilities|GetDataTableRow DataTable RowName)
    (:then
      (Widget|Panel|ClearChildren (Variables|/Game/Dialogue/WB_Dialogue.WB_Dialogue_C|GetOptionScrollBox (Variables|Default|GetDialogueWidget)))
      (Development|PrintString (Utilities|GetDisplayName (Variables|Default|GetAttachedActor)))
      (Default|UpdateDialogue (Variables|Default|GetDialogueWidget) (.Dialogue (Utilities|Struct|BreakDialogue_Structure _returnvalue)))
      (Variables|Default|SetRow%20Name (.Row (Utilities|Struct|BreakDialogue_Structure _returnvalue)))
      (Variables|Default|SetData%20Table (.DataTable (Utilities|Struct|BreakDialogue_Structure _returnvalue)))
      (Variables|Default|SetEndDialogue (.EndDialogue (Utilities|Struct|BreakDialogue_Structure _returnvalue))))))

(event EventInteraction
  (params (playerRef :type BP%20Third%20Person%20Character%20Object%20Reference))
  (bind _returnvalue (Game|GetPlayerController 0))
  (bind _returnvalue_2 (Game|GetPlayerController 0))
  ;[0.15 0.15 0.15 0.5] Create Dialogue on interactions
  (if (Variables|Default|GetEndDialogue)
    ;;[0.15 0 0 0.5] If the prior called line had end dialogue tag, instead of displaying a new line remove the widget, reset end dialogue/dialogue widget, and remove the cursor from the screen
    (Widget|RemovefromParent (Variables|Default|GetDialogueWidget))
    (Variables|Default|SetEndDialogue false)
    (Variables|Default|SetDialogueWidget 0)
    (Input|SetInputModeGameOnly _returnvalue false)
    (Variables|/Script/Engine.PlayerController|SetbShowMouseCursor _returnvalue false)
    (else
      (Utilities|IsValid (Variables|Default|GetDialogueWidget)
        (:Is%20Valid
          ;;[0.15 0 0.1035 0.5] If dialogue widget is valid and the prior line wasn't the last, get a specific row from the data table, update the dialogue with that row, and then update the data table/row name/end dialogue tags
          (bind _returnvalue_3 (Utilities|GetDataTableRow (Variables|Default|GetData%20Table) (Variables|Default|GetRow%20Name))
            (:then
              (Default|UpdateDialogue (Variables|Default|GetDialogueWidget) (.Dialogue (Utilities|Struct|BreakDialogue_Structure _returnvalue_3)))
              (Variables|Default|SetRow%20Name (.Row (Utilities|Struct|BreakDialogue_Structure _returnvalue_3)))
              (Variables|Default|SetData%20Table (.DataTable (Utilities|Struct|BreakDialogue_Structure _returnvalue_3)))
              (Variables|Default|SetEndDialogue (.EndDialogue (Utilities|Struct|BreakDialogue_Structure _returnvalue_3))))))
        (:Is%20Not%20Valid
          ;;[0 0.15 0.001164 0.5] If dialogue widjet is not valid, then create a dialogue widget
          (bind _returnvalue_4 (Utilities|GetDataTableRow (Variables|Default|GetData%20Table) (Variables|Default|GetRow%20Name))
            (:then
              (bind _returnvalue_5 (UserInterface|CreateWidget "/Game/Dialogue/WB_Dialogue.WB_Dialogue_C" 0 (Utilities|Text|ToText(Name) (Variables|Default|GetName)) (.Dialogue (Utilities|Struct|BreakDialogue_Structure _returnvalue_4))))
              (bind _output_get (Variables|Default|SetDialogueWidget _returnvalue_5))
              (Variables|Default|SetAttachedActor (Components|GetOwner))
              (UserInterface|Viewport|AddtoViewport _output_get 0)
              (Variables|Default|SetRow%20Name (.Row (Utilities|Struct|BreakDialogue_Structure _returnvalue_4)))
              (Variables|Default|SetData%20Table (.DataTable (Utilities|Struct|BreakDialogue_Structure _returnvalue_4)))
              (Variables|Default|SetEndDialogue (.EndDialogue (Utilities|Struct|BreakDialogue_Structure _returnvalue_4)))
              (Input|SetInputModeGameandUI _returnvalue_2 0 "DoNotLock" true false)
              (Variables|/Script/Engine.PlayerController|SetbShowMouseCursor _returnvalue_2 true)
              ;;[0 0.01718 0.15 0.5] If the dialogue from the data table has available options, create the options widgets
              (if (.OpenEndedDialogue (Utilities|Struct|BreakDialogue_Structure _returnvalue_4))
                (for _array_element (.OpenEndedDialogueOptions (Utilities|Struct|BreakDialogue_Structure _returnvalue_4))
                  (bind _returnvalue_6 (UserInterface|CreateWidget "/Game/Dialogue/WB_Option.WB_Option_C" 0 (Utilities|Text|ToText(Name) (.OptionName (Utilities|Struct|BreakOptionsDialogue_Structure _array_element))) self (.DataTable (Utilities|Struct|BreakOptionsDialogue_Structure _array_element)) (.Row (Utilities|Struct|BreakOptionsDialogue_Structure _array_element))))
                  (Widget|Panel|AddChild (Variables|/Game/Dialogue/WB_Dialogue.WB_Dialogue_C|GetOptionScrollBox (Variables|Default|GetDialogueWidget)) _returnvalue_6))))))))))

(event EventLeaveDialogue
  (bind _returnvalue (Game|GetPlayerController 0))
  ;[0.15 0.15 0.15 0.5] If Leave Dialogue is called, remove the choices dialogue widget
  ;[0.15 0.15 0.15 0.5] Create Dialogue on interactions
  (Utilities|IsValid (Variables|Default|GetDialogueWidget)
    (:Is%20Valid
      ;;[0.15 0 0 0.5] If the prior called line had end dialogue tag, instead of displaying a new line remove the widget, reset end dialogue/dialogue widget, and remove the cursor from the screen
      (Widget|RemovefromParent (Variables|Default|GetDialogueWidget))
      (Variables|Default|SetEndDialogue false)
      (Variables|Default|SetDialogueWidget 0)
      (Input|SetInputModeGameOnly _returnvalue false)
      (Variables|/Script/Engine.PlayerController|SetbShowMouseCursor _returnvalue false))))