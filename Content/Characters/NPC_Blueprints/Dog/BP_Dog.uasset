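; Dog NPC character that follows the player around once triggered.
; Trigger number 2 teleports the dog beside the player, then starts following after a short delay.
; FollowPlayer sets walk speed and loops AIMoveTo on the player's current location, repeating immediately on success or after a pause on failure.
; SidewalkWalk only sets walk speed, despite its comment describing pacing.
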(event Custom|Follow%20Player
  (Variables|/Script/Engine.CharacterMovementComponent|SetMaxWalkSpeed (Variables|Character|GetCharacterMovement) 1.5e+02)
  (bind _output_get (Variables|Default|SetPlayerLocation (Transformation|GetActorLocation (Game|Player|GetPlayerPawn 0))))
  (AI|AIMoveTo self _output_get 0 1e+02 false
    (:OnSuccess
      (CallFunction|FollowPlayer))
    (:OnFail
      (Utilities|FlowControl|Delay 1.0)
      (CallFunction|FollowPlayer))))

(event Custom|Sidewalk%20Walk
  ;[0.15 0.15 0.15 0.5] Set the NPC to walk to a public destination. On success beging pacing
  (Variables|/Script/Engine.CharacterMovementComponent|SetMaxWalkSpeed (Variables|Character|GetCharacterMovement) 1.5e+02))

(event EventBeginPlay)

(event EventTrigger
  (params (TriggerNum :type Integer))
  (bind _returnvalue (Game|Player|GetPlayerPawn 0))
  (bind _returnvalue_2 (Transformation|GetActorLocation _returnvalue))
  (bind (_x _y _z) (Math|Vector|BreakVector _returnvalue_2))
  (switch int TriggerNum
    (:2
      (Transformation|Teleport (Math|Vector|MakeVector _x (+ _y 1e+02) (- _z 2.5)) "0, 0, 0")
      (Utilities|FlowControl|Delay 2.0)
      (CallFunction|FollowPlayer))))

(fn ConstructionScript)