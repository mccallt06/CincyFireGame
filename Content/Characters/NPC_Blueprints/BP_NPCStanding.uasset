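; BP_NPCStanding is a stationary NPC with a dialogue component and interaction icons that reflect whether the player is nearby.
; Box overlap with the player swaps the outer icon for the inner one, and the construction script sizes and positions both.
; Its Trigger event switches the dialogue DataTable to DT_Pedestrian2 on 3 and forwards 4 and 5 to the BP_ItemText actor found in the level.
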(event OnComponentBeginOverlap(Box)
  (params (OverlappedComponent :type Primitive%20Component%20Object%20Reference) (OtherActor :type Actor%20Object%20Reference) (OtherComp :type Primitive%20Component%20Object%20Reference) (OtherBodyIndex :type Integer) (bFromSweep :type Boolean) (SweepResult :type Hit%20Result%20Structure%20%28by%20ref%29))
  ;[0.15 0.15 0.15 0.5] Display Inner/Outer icons
  (if (== OtherActor (Game|GetPlayerCharacter 0))
    (Development|SetHiddeninGame (Variables|Default|GetInnerIcon) false false)
    (Development|SetHiddeninGame (Variables|Default|GetOuterIcon) true false)))

(event OnComponentEndOverlap(Box)
  (params (OverlappedComponent :type Primitive%20Component%20Object%20Reference) (OtherActor :type Actor%20Object%20Reference) (OtherComp :type Primitive%20Component%20Object%20Reference) (OtherBodyIndex :type Integer))
  ;[0.15 0.15 0.15 0.5] Display Inner/Outer icons
  (if (== (Game|GetPlayerCharacter 0) OtherActor)
    (Development|SetHiddeninGame (Variables|Default|GetInnerIcon) true false)
    (Development|SetHiddeninGame (Variables|Default|GetOuterIcon) false false)))

(event EventTrigger
  (params (TriggerNum :type Integer))
  ;[0.15 0.15 0.15 0.5] Trigger Control System. On trigger 1 (conversation exit) reenable NPC movement. On trigger 2 (conversation enter) disable NPC movement. On trigger 3 switch data tables to the toy found variation.
  (switch int TriggerNum
    (:3
      (Variables|/Game/Dialogue/BP_DialogueComponent.BP_DialogueComponent_C|SetData%20Table (Variables|Default|GetBP_DialogueComponent) "/Game/Dialogue/DataTables/DT_Pedestrian2.DT_Pedestrian2"))
    (:4
      (bind _returnvalue (Actor|GetActorOfClass "/Game/UI/ItemText/BP_ItemText.BP_ItemText_C"))
      (Default|Trigger _returnvalue 4))
    (:5
      (bind _returnvalue_2 (Actor|GetActorOfClass "/Game/UI/ItemText/BP_ItemText.BP_ItemText_C"))
      (Default|Trigger _returnvalue_2 5))))

(fn ConstructionScript
  ;[0.15 0.15 0.15 0.5] Set Icon Size
  (Transformation|SetWorldScale3D (Variables|Default|GetInnerIcon) (Math|Conversions|ToVector(Float) (/ (Variables|Default|GetIconSize) 1e+01)))
  ;[0.15 0.15 0.15 0.5] Set front Icon Location
  (Transformation|SetRelativeLocation (Variables|Default|GetOuterIcon) (Variables|Default|GetIconLocation) false false))

(fn BPThirdPersonCharacterAutoGenFunc)