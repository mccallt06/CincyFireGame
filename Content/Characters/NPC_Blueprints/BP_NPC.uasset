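; Sidewalk NPC that walks to a destination, then paces back and forth so the player can talk to it from the balcony.
; AIMoveTo chains loop the pacing and flip the interaction box's side at each turn, while box overlaps swap inner and outer icons.
; Trigger events halt or resume movement for conversations, with a timeline turning the mesh toward or away from the player.
; The construction script sizes and positions the icons.
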(event OnComponentBeginOverlap(Box)
  (params (OverlappedComponent :type Primitive%20Component%20Object%20Reference) (OtherActor :type Actor%20Object%20Reference) (OtherComp :type Primitive%20Component%20Object%20Reference) (OtherBodyIndex :type Integer) (bFromSweep :type Boolean) (SweepResult :type Hit%20Result%20Structure%20%28by%20ref%29))
  ;[0.15 0.15 0.15 0.5] Display Inner/Outer icons
  (if (== OtherActor (Game|GetPlayerCharacter 0))
    (Development|SetHiddeninGame (Variables|Default|GetInnerIcon) false false)
    (Development|SetHiddeninGame (Variables|Default|GetOuterIcon) true false)))

(event OnComponentEndOverlap(Box)
  (params (OverlappedComponent :type Primitive%20Component%20Object%20Reference) (OtherActor :type Actor%20Object%20Reference) (OtherComp :type Primitive%20Component%20Object%20Reference) (OtherBodyIndex :type Integer))
  ;[0.15 0.15 0.15 0.5] Display Inner/Outer icons
  (if (== (Game|GetPlayerCharacter 0) OtherActor)
    (Development|SetHiddeninGame (Variables|Default|GetInnerIcon) true false)
    (Development|SetHiddeninGame (Variables|Default|GetOuterIcon) false false)))

(event Custom|SidewalkWalk
  ;[0.15 0.15 0.15 0.5] Set the NPC to walk to a public destination. On success beging pacing
  (Variables|/Script/Engine.CharacterMovementComponent|SetMaxWalkSpeed (Variables|Character|GetCharacterMovement) 1.5e+02)
  (AI|AIMoveTo self (Variables|Default|GetDestination) 0 5.0 false
    (:OnSuccess
      (CallFunction|Pacing))))

(event Custom|Pacing
  ;[0.15 0.15 0.15 0.5] Tells the NPC to walk back and forth and mvoes an interactable box with them (flipping sides each time) so that the player can talk to them from the balcony
  (Transformation|SetRelativeLocation (Variables|Default|GetBox) (- (Variables|/Script/Engine.SceneComponent|GetRelativeLocation (Variables|Default|GetBox)) "0.000000,1372.000000,0.000000") false false)
  (Variables|Default|SetWalkingBack true :!label _label)
  (AI|AIMoveTo self (+ (Variables|Default|GetDestination) (Math|Vector|MakeVector (Math|Random|RandomFloatinRange 5e+02 7.5e+02) 0.0 0.0)) 0 5.0 false
    (:OnSuccess
      (Transformation|SetRelativeLocation (Variables|Default|GetBox) (+ (Variables|/Script/Engine.SceneComponent|GetRelativeLocation (Variables|Default|GetBox)) "0.000000,1372.000000,0.000000") false false)
      (Variables|Default|SetWalkingBack false)
      (AI|AIMoveTo self (Variables|Default|GetDestination) 0 5.0 false
        (:OnSuccess
          (Transformation|SetRelativeLocation (Variables|Default|GetBox) (- (Variables|/Script/Engine.SceneComponent|GetRelativeLocation (Variables|Default|GetBox)) "0.000000,1372.000000,0.000000") false false)
          (goto _label))))))

(event EventBeginPlay
  (CallFunction|SidewalkWalk))

(event EventTrigger
  (params (TriggerNum :type Integer))
  (bind _returnvalue (Game|GetPlayerCharacter 0))
  (bind _charactermovement (Variables|Character|GetCharacterMovement))
  (bind _mesh (Variables|Character|GetMesh))
  (bind _mesh_2 (Variables|Character|GetMesh))
  (bind _charactermovement_2 (Variables|Character|GetCharacterMovement))
  (bind _returnvalue_2 (Transformation|GetActorLocation _returnvalue))
  (bind _returnvalue_3 (Transformation|GetWorldLocation _mesh_2))
  (bind _returnvalue_4 (Math|Rotator|FindLookatRotation _returnvalue_3 _returnvalue_2))
  (bind _returnvalue_5 (+ (.yaw _returnvalue_4) 2.7e+02))
  (bind _returnvalue_6 (Math|Rotator|MakeRotator 0.0 0.0 _returnvalue_5))
  ;[0.15 0.15 0.15 0.5] Trigger Control System. On trigger 1 (conversation exit) reenable NPC movement. On trigger 2 (conversation enter) disable NPC movement
  (switch int TriggerNum
    (:1
      (Variables|/Script/Engine.CharacterMovementComponent|SetMaxWalkSpeed _charactermovement_2 1.5e+02)
      (Pawn|Components|CharacterMovement|SetMovementMode _charactermovement_2 "MOVE_Walking" 0)
      (bind _newtrack_0 (Timeline|Timeline ReverseFromEnd)
        (:Update
          (if (Variables|Default|GetWalkingBack)
            (Transformation|SetWorldRotation _mesh (Math|Rotator|Lerp(Rotator) (Variables|Default|GetStartRotation) (Math|Rotator|MakeRotator 0.0 0.0 (- (.yaw _returnvalue_4) 9e+01)) _newtrack_0) false false)
            (else
              (Transformation|SetWorldRotation _mesh (Math|Rotator|Lerp(Rotator) "0.000000,90.000000,0.000000" _returnvalue_6 _newtrack_0 true) false false)
              (Variables|Default|SetCurrentRotation (Math|Rotator|Lerp(Rotator) "0.000000,90.000000,0.000000" _returnvalue_6 _newtrack_0 true))
              (Utilities|FlowControl|Delay 1e+01)
              (if (== 0.0 (Math|Vector|VectorLength (Pawn|Components|CharacterMovement|GetLastUpdateVelocity (Variables|Character|GetCharacterMovement))))
                (CallFunction|Pacing)))))))
    (:2
      (Variables|/Script/Engine.CharacterMovementComponent|SetMaxWalkSpeed _charactermovement 0.0)
      (Variables|Default|SetStartRotation (Transformation|GetWorldRotation _mesh_2))
      (Pawn|Components|CharacterMovement|DisableMovement _charactermovement)
      (if (Utilities|Operators|NotEqual(!=) (Variables|Default|GetCurrentRotation) _returnvalue_6 0.0)
        (Timeline|Timeline PlayFromStart)))))

(fn ConstructionScript
  ;[0.15 0.15 0.15 0.5] Set Icon Size
  (Transformation|SetWorldScale3D (Variables|Default|GetInnerIcon) (Math|Conversions|ToVector(Float) (/ (Variables|Default|GetIconSize) 1e+01)))
  ;[0.15 0.15 0.15 0.5] Set front Icon Location
  (Transformation|SetRelativeLocation (Variables|Default|GetOuterIcon) (Variables|Default|GetIconLocation) false false))

(fn BPThirdPersonCharacterAutoGenFunc)