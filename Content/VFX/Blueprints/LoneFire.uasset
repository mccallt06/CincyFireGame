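; LoneFire is a fire hazard actor that, when triggered, places fire at the player's position and damages the player while inside it.
; Trigger moves the Niagara effect slightly above the player's origin, adds a scaled sphere collision there, then nudges the player after a short delay to force overlap detection.
; Begin and end overlap toggle an InFire flag, which drives a delay loop applying repeated damage.
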(event Collision|EventActorBeginOverlap
  (params (OtherActor :type Actor%20Object%20Reference))
  ;[0.15 0.15 0.15 0.5] If player is standing in fire, deal 5 damage to them. If still in it .2 seconds later, repeat.
  (if (== OtherActor (Game|GetPlayerCharacter 0))
    (Variables|Default|SetInFire true)
    (Game|Damage|ApplyDamage OtherActor 5.0 0 0 :!label _label)
    (Utilities|FlowControl|Delay 0.2)
    (if (Variables|Default|GetInFire)
      (goto _label))))

(event Collision|EventActorEndOverlap
  (params (OtherActor :type Actor%20Object%20Reference))
  ;[0.15 0.15 0.15 0.5] SetsPlayer as no longer in the fire once the overlap ends
  (Variables|Default|SetInFire false))

(event EventTrigger
  (params (TriggerNum :type Integer))
  (bind _returnvalue (Game|GetPlayerCharacter 0))
  (bind _returnvalue_2 (Game|GetPlayerCharacter 0))
  (bind _returnvalue_3 (Transformation|GetActorLocation _returnvalue_2))
  (bind (_x _y _z) (Math|Vector|BreakVector _returnvalue_3))
  (bind _returnvalue_4 (+ _z 9e+01))
  ;[0.15 0.15 0.15 0.5] Upon recieving an event trigger, spawn fire on the players location, add a sphere collision to it, then slightly move the player to force the system to recognize that the player is in the fire.
  (Transformation|SetWorldLocation (Variables|Default|GetNiagara) (Math|Vector|MakeVector _x _y _returnvalue_4) false false)
  (AddComponent|AddSphereComponent true (Math|Transform|MakeTransform (Math|Vector|MakeVector _x _y _returnvalue_4) "0, 0, 0" "2.000000,2.000000,2.000000"))
  (Utilities|FlowControl|Delay 0.2)
  (Transformation|SetActorLocation _returnvalue (+ (Transformation|GetActorLocation _returnvalue) "0.000000,0.100000,0.000000") false false))

(fn ConstructionScript)