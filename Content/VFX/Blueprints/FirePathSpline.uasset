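; Fire hazard that spreads along a spline and repeatedly damages the player while they overlap it.
; A self-restarting timeline steps along the spline, spawning Niagara fire and sound until the next point is too close to the last.
; A second timeline consumes the recorded points to add sphere collision components at runtime.
; Spreading starts after a BeginPlay delay, stopping and resuming on the player character's text enter and exit events.
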(event Custom|StartFire
  ;[0.15 0.15 0.15 0.5] Spawns fires along the path of a spline
  (Utilities|FlowControl|Sequence
    (:then_0
      (Timeline|Timeline_0 Play
        (:Finished
          (if (Utilities|Operators|EqualEqual (Variables|Default|GetPreviousPoint) (Spline|GetLocationatDistanceAlongSpline (Variables|Default|GetSpline) (Variables|Default|GetFireDistanceHolder) "World") 2.5e+02)
            (CallFunction|StopFires)
            (else
              (bind _returnvalue (Niagara|SpawnSystematLocation (Variables|Default|GetNiagaraFire) (Spline|GetLocationatDistanceAlongSpline (Variables|Default|GetSpline) (Variables|Default|GetFireDistanceHolder) "World") "0, 0, 0" "12.000000,12.000000,12.000000" false true "None" false))
              (Audio|SpawnSoundatLocation "/Game/StarterContent/Audio/Fire01_Cue.Fire01_Cue" (Spline|GetLocationatDistanceAlongSpline (Variables|Default|GetSpline) (Variables|Default|GetFireDistanceHolder) "World") "0, 0, 0" 1.0 1.0 0.0 0 0)
              (Utilities|Array|Add (Variables|Default|GetFireEffectsArray) _returnvalue)
              (bind _output_get (Variables|Default|SetPreviousPoint (Spline|GetLocationatDistanceAlongSpline (Variables|Default|GetSpline) (Variables|Default|GetFireDistanceHolder) "World")))
              (Utilities|Array|Add (Variables|Default|GetPreviousPointsArray) _output_get)
              (Variables|Default|SetFireDistanceHolder (+ (Variables|Default|GetFireDistance) (Variables|Default|GetFireDistanceHolder)))
              (CallFunction|RestartFire))))))
    (:then_1
      (Utilities|FlowControl|Delay 0.2)
      (CallFunction|StartCollsions))))

(event Custom|StopFires
  ;[0.15 0.15 0.15 0.5] Spawns fires along the path of a spline
  (Timeline|Timeline_0 Stop
    (:Finished
      (if (Utilities|Operators|EqualEqual (Variables|Default|GetPreviousPoint) (Spline|GetLocationatDistanceAlongSpline (Variables|Default|GetSpline) (Variables|Default|GetFireDistanceHolder) "World") 2.5e+02)
        (CallFunction|StopFires)
        (else
          (bind _returnvalue (Niagara|SpawnSystematLocation (Variables|Default|GetNiagaraFire) (Spline|GetLocationatDistanceAlongSpline (Variables|Default|GetSpline) (Variables|Default|GetFireDistanceHolder) "World") "0, 0, 0" "12.000000,12.000000,12.000000" false true "None" false))
          (Audio|SpawnSoundatLocation "/Game/StarterContent/Audio/Fire01_Cue.Fire01_Cue" (Spline|GetLocationatDistanceAlongSpline (Variables|Default|GetSpline) (Variables|Default|GetFireDistanceHolder) "World") "0, 0, 0" 1.0 1.0 0.0 0 0)
          (Utilities|Array|Add (Variables|Default|GetFireEffectsArray) _returnvalue)
          (bind _output_get (Variables|Default|SetPreviousPoint (Spline|GetLocationatDistanceAlongSpline (Variables|Default|GetSpline) (Variables|Default|GetFireDistanceHolder) "World")))
          (Utilities|Array|Add (Variables|Default|GetPreviousPointsArray) _output_get)
          (Variables|Default|SetFireDistanceHolder (+ (Variables|Default|GetFireDistance) (Variables|Default|GetFireDistanceHolder)))
          (CallFunction|RestartFire))))))

(event Custom|StopCollisions
  (bind _previouspointsarray (Variables|Default|GetPreviousPointsArray))
  (bind _output (Utilities|Array|Get(acopy) _previouspointsarray))
  ;[0.15 0.15 0.15 0.5] Spawning Fire Collision
  (Timeline|CollsionSpawning Stop
    (:Update
      (Utilities|FlowControl|Delay (Variables|Default|GetTimeBetweenFires))
      (if (Utilities|Operators|EqualEqual _output (Variables|Default|GetPreviousCollision) 0.0)
        (CallFunction|StopCollisions)
        (else
          (bind _returnvalue (AddComponent|AddSphereComponent true (Math|Transform|MakeTransform _output "0, 0, 0" "2.000000,2.000000,2.000000")))
          (Collision|SetCollisionProfileName _returnvalue "None" true :!class /Script/Engine.PrimitiveComponent)
          (Variables|Default|SetPreviousCollision "0, 0, 0")
          (Utilities|Array|RemoveIndex (Variables|Default|GetPreviousPointsArray))
          (Utilities|Array|Add (Variables|Default|GetCollisionsArray) _returnvalue)
          (Utilities|FlowControl|DelayUntilNextTick)
          (Development|PrintString (Utilities|GetDisplayName (Utilities|Array|Get(acopy) (Collision|GetOverlappingActors _returnvalue "/Game/ThirdPerson/Blueprints/BP_ThirdPersonCharacter.BP_ThirdPersonCharacter_C" :!class /Script/Engine.PrimitiveComponent)))))))))

(event Custom|StartCollsions
  (bind _previouspointsarray (Variables|Default|GetPreviousPointsArray))
  (bind _output (Utilities|Array|Get(acopy) _previouspointsarray))
  ;[0.15 0.15 0.15 0.5] Spawning Fire Collision
  (Timeline|CollsionSpawning Play
    (:Update
      (Utilities|FlowControl|Delay (Variables|Default|GetTimeBetweenFires))
      (if (Utilities|Operators|EqualEqual _output (Variables|Default|GetPreviousCollision) 0.0)
        (CallFunction|StopCollisions)
        (else
          (bind _returnvalue (AddComponent|AddSphereComponent true (Math|Transform|MakeTransform _output "0, 0, 0" "2.000000,2.000000,2.000000")))
          (Collision|SetCollisionProfileName _returnvalue "None" true :!class /Script/Engine.PrimitiveComponent)
          (Variables|Default|SetPreviousCollision "0, 0, 0")
          (Utilities|Array|RemoveIndex (Variables|Default|GetPreviousPointsArray))
          (Utilities|Array|Add (Variables|Default|GetCollisionsArray) _returnvalue)
          (Utilities|FlowControl|DelayUntilNextTick)
          (Development|PrintString (Utilities|GetDisplayName (Utilities|Array|Get(acopy) (Collision|GetOverlappingActors _returnvalue "/Game/ThirdPerson/Blueprints/BP_ThirdPersonCharacter.BP_ThirdPersonCharacter_C" :!class /Script/Engine.PrimitiveComponent)))))))))

(event Custom|OnTextExited
  (CallFunction|StartFire))

(event Custom|OnTextEntered
  (CallFunction|StopFires)
  (CallFunction|StopCollisions))

(event Custom|RestartFire
  ;[0.15 0.15 0.15 0.5] Spawns fires along the path of a spline
  (Timeline|Timeline_0 PlayFromStart
    (:Finished
      (if (Utilities|Operators|EqualEqual (Variables|Default|GetPreviousPoint) (Spline|GetLocationatDistanceAlongSpline (Variables|Default|GetSpline) (Variables|Default|GetFireDistanceHolder) "World") 2.5e+02)
        (CallFunction|StopFires)
        (else
          (bind _returnvalue (Niagara|SpawnSystematLocation (Variables|Default|GetNiagaraFire) (Spline|GetLocationatDistanceAlongSpline (Variables|Default|GetSpline) (Variables|Default|GetFireDistanceHolder) "World") "0, 0, 0" "12.000000,12.000000,12.000000" false true "None" false))
          (Audio|SpawnSoundatLocation "/Game/StarterContent/Audio/Fire01_Cue.Fire01_Cue" (Spline|GetLocationatDistanceAlongSpline (Variables|Default|GetSpline) (Variables|Default|GetFireDistanceHolder) "World") "0, 0, 0" 1.0 1.0 0.0 0 0)
          (Utilities|Array|Add (Variables|Default|GetFireEffectsArray) _returnvalue)
          (bind _output_get (Variables|Default|SetPreviousPoint (Spline|GetLocationatDistanceAlongSpline (Variables|Default|GetSpline) (Variables|Default|GetFireDistanceHolder) "World")))
          (Utilities|Array|Add (Variables|Default|GetPreviousPointsArray) _output_get)
          (Variables|Default|SetFireDistanceHolder (+ (Variables|Default|GetFireDistance) (Variables|Default|GetFireDistanceHolder)))
          (CallFunction|RestartFire))))))

(event Collision|EventActorBeginOverlap
  (params (OtherActor :type Actor%20Object%20Reference))
  ;[0.15 0.15 0.15 0.5] If player is overlapping with the fire, take 5 damage. Repeat if they are still in the fire after the delay
  (if (== OtherActor (Game|GetPlayerCharacter 0))
    (Variables|Default|SetInFire true)
    (Game|Damage|ApplyDamage OtherActor 34.0 0 0 :!label _label)
    (Utilities|FlowControl|Delay 0.2)
    (if (Variables|Default|GetInFire)
      (Class|BPITrigger|Trigger(Message) (Game|GetPlayerCharacter 0) 10)
      (goto _label))))

(event Collision|EventActorEndOverlap
  (params (OtherActor :type Actor%20Object%20Reference))
  ;[0.15 0.15 0.15 0.5] SetsPlayer as no longer in the fire once the overlap ends
  (Variables|Default|SetInFire false))

(event EventBeginPlay
  (Utilities|FlowControl|Sequence
    (:then_0
      (Utilities|FlowControl|DelayUntilNextTick)
      (bind _returnvalue (Actor|GetActorOfClass "/Game/ThirdPerson/Blueprints/BP_ThirdPersonCharacter.BP_ThirdPersonCharacter_C"))
      (bind _output_get (Variables|Default|SetPlayerRef _returnvalue))
      (EventDispatchers|BindEventtoOnTextExited _output_get (EventDispatchers|CreateEvent :!event Custom|OnTextExited))
      (EventDispatchers|BindEventtoOnTextEntered _output_get (EventDispatchers|CreateEvent :!event Custom|OnTextEntered)))
    (:then_1
      (Utilities|FlowControl|Delay 2.0)
      (CallFunction|StartFire))))

(fn ConstructionScript)