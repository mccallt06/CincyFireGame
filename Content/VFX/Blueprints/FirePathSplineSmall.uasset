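; Blueprint that spreads Niagara fire effects along a spline, starting two seconds after BeginPlay.
; Timeline updates, throttled by a Delay, spawn fire at successive distances along the spline and store each effect and location.
; The timeline stops when the next location lies within a tolerance of the previous one, as happens when distance clamps at the spline's end.
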(event Custom|StartFire
  (Timeline|Timeline PlayFromStart
    (:Update
      (Utilities|FlowControl|Delay (Variables|Default|GetTimeBetweenFires))
      (if (Utilities|Operators|EqualEqual (Variables|Default|GetPreviousPoint) (Spline|GetLocationatDistanceAlongSpline (Variables|Default|GetSpline) (Variables|Default|GetFireDistanceHolder) "World") 2.5e+02)
        (CallFunction|StopFires)
        (else
          (bind _returnvalue (Niagara|SpawnSystematLocation (Variables|Default|GetNiagaraFire) (Spline|GetLocationatDistanceAlongSpline (Variables|Default|GetSpline) (Variables|Default|GetFireDistanceHolder) "World") "0, 0, 0" "1.000000,1.000000,1.000000" false true "None" false))
          (Utilities|Array|Add (Variables|Default|GetFireEffectsArray) _returnvalue)
          (bind _output_get (Variables|Default|SetPreviousPoint (Spline|GetLocationatDistanceAlongSpline (Variables|Default|GetSpline) (Variables|Default|GetFireDistanceHolder) "World")))
          (Utilities|Array|Add (Variables|Default|GetPreviousPointsArray) _output_get)
          (bind _output_get_2 (Variables|Default|SetFireDistanceHolder (+ (Variables|Default|GetFireDistance) (Variables|Default|GetFireDistanceHolder)))))))))

(event Custom|StopFires
  (Timeline|Timeline Stop
    (:Update
      (Utilities|FlowControl|Delay (Variables|Default|GetTimeBetweenFires))
      (if (Utilities|Operators|EqualEqual (Variables|Default|GetPreviousPoint) (Spline|GetLocationatDistanceAlongSpline (Variables|Default|GetSpline) (Variables|Default|GetFireDistanceHolder) "World") 2.5e+02)
        (CallFunction|StopFires)
        (else
          (bind _returnvalue (Niagara|SpawnSystematLocation (Variables|Default|GetNiagaraFire) (Spline|GetLocationatDistanceAlongSpline (Variables|Default|GetSpline) (Variables|Default|GetFireDistanceHolder) "World") "0, 0, 0" "1.000000,1.000000,1.000000" false true "None" false))
          (Utilities|Array|Add (Variables|Default|GetFireEffectsArray) _returnvalue)
          (bind _output_get (Variables|Default|SetPreviousPoint (Spline|GetLocationatDistanceAlongSpline (Variables|Default|GetSpline) (Variables|Default|GetFireDistanceHolder) "World")))
          (Utilities|Array|Add (Variables|Default|GetPreviousPointsArray) _output_get)
          (bind _output_get_2 (Variables|Default|SetFireDistanceHolder (+ (Variables|Default|GetFireDistance) (Variables|Default|GetFireDistanceHolder)))))))))

(event EventBeginPlay
  (Utilities|FlowControl|Delay 2.0)
  (CallFunction|StartFire))

(fn ConstructionScript)