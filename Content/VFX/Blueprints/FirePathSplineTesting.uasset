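; Test actor that lays a damaging trail of fire along a spline shortly after play begins.
; A timeline with delays steps along the spline spawning Niagara fire and sound, stopping when the next point falls near the previous one.
; A second, slightly delayed timeline consumes the recorded points to add lowered collision spheres.
; The player character takes repeated damage while overlapping the actor.
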(event Custom|StartFire
  ;[0.15 0.15 0.15 0.5] Spawns fires along the path of a spline
  (Utilities|FlowControl|Sequence
    (:then_0
      (Timeline|Timeline PlayFromStart
        (:Update
          (Utilities|FlowControl|Delay (Variables|Default|GetTimeBetweenFires))
          (if (Utilities|Operators|EqualEqual (Variables|Default|GetPreviousPoint) (Spline|GetLocationatDistanceAlongSpline (Variables|Default|GetSpline) (Variables|Default|GetFireDistanceHolder) "World") 2.5e+02)
            (CallFunction|StopFires)
            (else
              (bind _returnvalue (Niagara|SpawnSystematLocation (Variables|Default|GetNiagaraFire) (Spline|GetLocationatDistanceAlongSpline (Variables|Default|GetSpline) (Variables|Default|GetFireDistanceHolder) "World") "0, 0, 0" "1.000000,1.000000,1.000000" false true "None" false))
              (Audio|SpawnSoundatLocation "/Game/StarterContent/Audio/Fire01_Cue.Fire01_Cue" (Spline|GetLocationatDistanceAlongSpline (Variables|Default|GetSpline) (Variables|Default|GetFireDistanceHolder) "World") "0, 0, 0" 1.0 1.0 0.0 0 0)
              (Utilities|Array|Add (Variables|Default|GetFireEffectsArray) _returnvalue)
              (bind _output_get (Variables|Default|SetPreviousPoint (Spline|GetLocationatDistanceAlongSpline (Variables|Default|GetSpline) (Variables|Default|GetFireDistanceHolder) "World")))
              (Utilities|Array|Add (Variables|Default|GetPreviousPointsArray) _output_get)
              (Variables|Default|SetFireDistanceHolder (+ (Variables|Default|GetFireDistance) (Variables|Default|GetFireDistanceHolder))))))))
    (:then_1
      (Utilities|FlowControl|Delay 0.2)
      (CallFunction|StartCollsions))))

(event Custom|StopFires
  ;[0.15 0.15 0.15 0.5] Spawns fires along the path of a spline
  (Timeline|Timeline Stop
    (:Update
      (Utilities|FlowControl|Delay (Variables|Default|GetTimeBetweenFires))
      (if (Utilities|Operators|EqualEqual (Variables|Default|GetPreviousPoint) (Spline|GetLocationatDistanceAlongSpline (Variables|Default|GetSpline) (Variables|Default|GetFireDistanceHolder) "World") 2.5e+02)
        (CallFunction|StopFires)
        (else
          (bind _returnvalue (Niagara|SpawnSystematLocation (Variables|Default|GetNiagaraFire) (Spline|GetLocationatDistanceAlongSpline (Variables|Default|GetSpline) (Variables|Default|GetFireDistanceHolder) "World") "0, 0, 0" "1.000000,1.000000,1.000000" false true "None" false))
          (Audio|SpawnSoundatLocation "/Game/StarterContent/Audio/Fire01_Cue.Fire01_Cue" (Spline|GetLocationatDistanceAlongSpline (Variables|Default|GetSpline) (Variables|Default|GetFireDistanceHolder) "World") "0, 0, 0" 1.0 1.0 0.0 0 0)
          (Utilities|Array|Add (Variables|Default|GetFireEffectsArray) _returnvalue)
          (bind _output_get (Variables|Default|SetPreviousPoint (Spline|GetLocationatDistanceAlongSpline (Variables|Default|GetSpline) (Variables|Default|GetFireDistanceHolder) "World")))
          (Utilities|Array|Add (Variables|Default|GetPreviousPointsArray) _output_get)
          (Variables|Default|SetFireDistanceHolder (+ (Variables|Default|GetFireDistance) (Variables|Default|GetFireDistanceHolder))))))))

(event Custom|StopCollisions
  (bind _previouspointsarray (Variables|Default|GetPreviousPointsArray))
  (bind _output (Utilities|Array|Get(acopy) _previouspointsarray))
  (bind _returnvalue (+ _output "0.000000,0.000000,-80.000000"))
  ;[0.15 0.15 0.15 0.5] Spawning Fire Collision
  (Timeline|CollsionSpawning Stop
    (:Update
      (Utilities|FlowControl|Delay (Variables|Default|GetTimeBetweenFires))
      (if (not (Utilities|Operators|EqualEqual (Variables|Default|GetPreviousCollision) _returnvalue 0.0))
        (bind _returnvalue_2 (AddComponent|AddSphereComponent true (Math|Transform|MakeTransform _returnvalue "0, 0, 0" "2.000000,2.000000,2.000000")))
        (Variables|Default|SetPreviousCollision _returnvalue)
        (Utilities|Array|RemoveIndex (Variables|Default|GetPreviousPointsArray))
        (Utilities|Array|Add (Variables|Default|GetCollisionsArray) _returnvalue_2)))))

(event Custom|StartCollsions
  (bind _previouspointsarray (Variables|Default|GetPreviousPointsArray))
  (bind _output (Utilities|Array|Get(acopy) _previouspointsarray))
  (bind _returnvalue (+ _output "0.000000,0.000000,-80.000000"))
  ;[0.15 0.15 0.15 0.5] Spawning Fire Collision
  (Timeline|CollsionSpawning PlayFromStart
    (:Update
      (Utilities|FlowControl|Delay (Variables|Default|GetTimeBetweenFires))
      (if (not (Utilities|Operators|EqualEqual (Variables|Default|GetPreviousCollision) _returnvalue 0.0))
        (bind _returnvalue_2 (AddComponent|AddSphereComponent true (Math|Transform|MakeTransform _returnvalue "0, 0, 0" "2.000000,2.000000,2.000000")))
        (Variables|Default|SetPreviousCollision _returnvalue)
        (Utilities|Array|RemoveIndex (Variables|Default|GetPreviousPointsArray))
        (Utilities|Array|Add (Variables|Default|GetCollisionsArray) _returnvalue_2)))))

(event Collision|EventActorBeginOverlap
  (params (OtherActor :type Actor%20Object%20Reference))
  ;[0.15 0.15 0.15 0.5] If player is overlapping with the fire, take 5 damage. Repeat if they are still in the fire after the delay
  (if (== OtherActor (Game|GetPlayerCharacter 0))
    (Variables|Default|SetInFire true)
    (Game|Damage|ApplyDamage OtherActor 5.0 0 0 :!label _label)
    (Utilities|FlowControl|Delay 0.2)
    (if (Variables|Default|GetInFire)
      (goto _label))))

(event Collision|EventActorEndOverlap
  (params (OtherActor :type Actor%20Object%20Reference))
  ;[0.15 0.15 0.15 0.5] SetsPlayer as no longer in the fire once the overlap ends
  (Variables|Default|SetInFire false))

(event EventBeginPlay
  ;[0.15 0.15 0.15 0.5] Spawns fires along the path of a spline
  (Utilities|FlowControl|Delay 2.0)
  (CallFunction|StartFire))

(fn ConstructionScript)