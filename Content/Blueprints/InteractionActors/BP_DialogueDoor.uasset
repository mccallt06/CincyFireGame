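; Interactable door that starts dialogue through BPDialogueComponent and opens or closes in response to numbered dialogue triggers.
; Triggers either spawn LoneFire at the player or swap the open/closed dialogue table and notify BP_DialogueWindow.
; A FlipFlop plays or reverses a timeline, using a cross product to swing the door away from the player.
; Radius overlaps switch inner and outer icons on both sides, which shift as the door swings.
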(event OnComponentBeginOverlap(InnerIconRadius)
  (params (OverlappedComponent :type Primitive%20Component%20Object%20Reference) (OtherActor :type Actor%20Object%20Reference) (OtherComp :type Primitive%20Component%20Object%20Reference) (OtherBodyIndex :type Integer) (bFromSweep :type Boolean) (SweepResult :type Hit%20Result%20Structure%20%28by%20ref%29))
  ;[0.15 0.15 0.15 0.5] Display Inner/Outer icons
  (if (== OtherActor (Game|GetPlayerCharacter 0))
    (Development|SetHiddeninGame (Variables|Default|GetInnerIcon) false false)
    (Development|SetHiddeninGame (Variables|Default|GetOuterIcon) true false)))

(event OnComponentEndOverlap(InnerIconRadius)
  (params (OverlappedComponent :type Primitive%20Component%20Object%20Reference) (OtherActor :type Actor%20Object%20Reference) (OtherComp :type Primitive%20Component%20Object%20Reference) (OtherBodyIndex :type Integer))
  ;[0.15 0.15 0.15 0.5] Display Inner/Outer icons
  (if (== (Game|GetPlayerCharacter 0) OtherActor)
    (Development|SetHiddeninGame (Variables|Default|GetInnerIcon) true false)
    (Development|SetHiddeninGame (Variables|Default|GetOuterIcon) false false)))

(event OnComponentBeginOverlap(OuterIconRadius)
  (params (OverlappedComponent :type Primitive%20Component%20Object%20Reference) (OtherActor :type Actor%20Object%20Reference) (OtherComp :type Primitive%20Component%20Object%20Reference) (OtherBodyIndex :type Integer) (bFromSweep :type Boolean) (SweepResult :type Hit%20Result%20Structure%20%28by%20ref%29))
  ;[0.15 0.15 0.15 0.5] Display Inner/Outer icons
  (if (== OtherActor (Game|GetPlayerCharacter 0))
    (Development|SetHiddeninGame (Variables|Default|GetOuterIcon) false false)))

(event OnComponentEndOverlap(OuterIconRadius)
  (params (OverlappedComponent :type Primitive%20Component%20Object%20Reference) (OtherActor :type Actor%20Object%20Reference) (OtherComp :type Primitive%20Component%20Object%20Reference) (OtherBodyIndex :type Integer))
  ;[0.15 0.15 0.15 0.5] Display Inner/Outer icons
  (if (== (Game|GetPlayerCharacter 0) OtherActor)
    (Development|SetHiddeninGame (Variables|Default|GetOuterIcon) true false)))

(event Custom|OpenCloseDoor
  ;[0.15 0.15 0.15 0.5] Open/Close door
  (Audio|PlaySoundatLocation "/Game/Audio/SFX/SFX/SFX_OpenCloseDoor.SFX_OpenCloseDoor" (Transformation|GetActorLocation (Game|GetPlayerCharacter 0)) "0, 0, 0" 1.0 1.0 0.0 0 0 0 0)
  (Utilities|FlowControl|FlipFlop
    (:A
      (Variables|Default|SetRotation (Math|Float|SelectFloat 85.0 -85.0 (>= (.z (Math|Vector|CrossProduct (Math|Vector|GetUnitDirection(Vector) (Transformation|GetActorLocation) (Transformation|GetActorLocation (Game|GetPlayerCharacter 0))) (Transformation|GetActorForwardVector))) 0.0)))
      (bind _alpha (Timeline|Door_TL Play)
        (:Update
          (Transformation|SetRelativeRotation (Variables|Default|GetDoor) (Math|Rotator|MakeRotator 0.0 0.0 (Math|Float|Lerp 0.0 (Variables|Default|GetRotation) _alpha)) false false)
          ;[0.15 0.15 0.15 0.5] Move the inner/outer icons
          (Transformation|SetRelativeLocation (Variables|Default|GetInnerIcon) (Math|Vector|MakeVector 0.0 (Math|Float|Lerp -2e+01 0.0 _alpha) 5e+01) false false)
          (Transformation|SetRelativeLocation (Variables|Default|GetInnerIconOpposite) (Math|Vector|MakeVector 0.0 (Math|Float|Lerp 2e+01 0.0 _alpha) 5e+01) false false))))
    (:B
      (Timeline|Door_TL Reverse))))

(event EventBeginPlay
  ;[0.15 0.15 0.15 0.5] Create player reference
  (bind _asbp_third_person_character (Utilities|Casting|CastToBP_ThirdPersonCharacter (Game|GetPlayerCharacter 0)))
  (Variables|Default|SetPlayerRef _asbp_third_person_character))

(event EventTrigger
  (params (TriggerNum :type Integer))
  (bind _returnvalue (Game|GetPlayerCharacter 0))
  (bind _returnvalue_2 (Transformation|GetActorLocation _returnvalue))
  ;[0.15 0.15 0.15 0.5] Trigger Switch for dialogue door. Trigger 1 goes to BP_LoneFire.
  (switch int TriggerNum
    (:2
      (bind _returnvalue_3 (Actor|GetActorOfClass "/Game/VFX/Blueprints/LoneFire.LoneFire_C"))
      (Default|SpawnFire _returnvalue_3 (Math|Vector|MakeVector (.x _returnvalue_2) (.y _returnvalue_2) (- (.z _returnvalue_2) 6e+01)))
      (Default|LeaveDialogue (Variables|Default|GetBP_DialogueComponent self))
      (CallFunction|OpenCloseDoor))
    (:3
      (Default|LeaveDialogue (Variables|Default|GetBP_DialogueComponent self))
      (CallFunction|OpenCloseDoor)
      (if (Variables|Default|GetDoorClosed)
        (Variables|Default|SetDoorClosed false)
        (Variables|/Game/Dialogue/BP_DialogueComponent.BP_DialogueComponent_C|SetData%20Table (Variables|Default|GetBP_DialogueComponent) "/Game/Dialogue/DataTables/DT_BedroomDoorOpen.DT_BedroomDoorOpen")
        (bind _returnvalue_4 (Actor|GetActorOfClass "/Game/Blueprints/InteractionActors/BP_DialogueWindow.BP_DialogueWindow_C"))
        (Default|Trigger _returnvalue_4 5)
        (else
          (Variables|Default|SetDoorClosed true)
          (Variables|/Game/Dialogue/BP_DialogueComponent.BP_DialogueComponent_C|SetData%20Table (Variables|Default|GetBP_DialogueComponent) "/Game/Dialogue/DataTables/DT_BedroomDoor.DT_BedroomDoor")
          (bind _returnvalue_5 (Actor|GetActorOfClass "/Game/Blueprints/InteractionActors/BP_DialogueWindow.BP_DialogueWindow_C"))
          (Default|Trigger _returnvalue_5 6))))))

(event EventInteraction
  (params (playerRef :type BP%20Third%20Person%20Character%20Object%20Reference))
  ;[0.15 0.15 0.15 0.5] Open/Close door
  (Development|PrintString "DOOR INTERACTED")
  (Default|Interaction (Variables|Default|GetBP_DialogueComponent self) (Variables|Default|GetPlayerRef)))

(fn ConstructionScript
  ;[0.15 0.15 0.15 0.5] Set Icon Size
  (Transformation|SetWorldScale3D (Variables|Default|GetInnerIcon) (Math|Conversions|ToVector(Float) (/ (Variables|Default|GetIconSize) 1e+01)))
  ;[0.15 0.15 0.15 0.5] Set front Icon Location
  (Transformation|SetRelativeLocation (Variables|Default|GetOuterIcon) (Variables|Default|GetIconLocation) false false)
  ;[0.15 0.15 0.15 0.5] Set Icon location for opposite side
  (Transformation|SetRelativeLocation (Variables|Default|GetInnerIconOpposite) (Variables|Default|GetItemLocationBack) false false))