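; Dialogue-gated door actor that swings open or shut when its Trigger event receives the matching number, while its own Interaction event is empty.
; That trigger messages the LoneFire actor, leaves the BPDialogueComponent conversation, then flip-flops a timeline that rotates the door and slides its icons.
; Two overlap radii swap outer and inner prompt icons on both sides as the player approaches, with size and placement set at construction.
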(event OnComponentBeginOverlap(InnerIconRadius)
  (params (OverlappedComponent :type Primitive%20Component%20Object%20Reference) (OtherActor :type Actor%20Object%20Reference) (OtherComp :type Primitive%20Component%20Object%20Reference) (OtherBodyIndex :type Integer) (bFromSweep :type Boolean) (SweepResult :type Hit%20Result%20Structure%20%28by%20ref%29))
  ;[0.15 0.15 0.15 0.5] Display Inner/Outer icons
  (if (== OtherActor (Game|GetPlayerCharacter 0))
    (Development|SetHiddeninGame (Variables|Default|GetInnerIcon) false false)
    (Development|SetHiddeninGame (Variables|Default|GetOuterIcon) true false)))

(event OnComponentEndOverlap(InnerIconRadius)
  (params (OverlappedComponent :type Primitive%20Component%20Object%20Reference) (OtherActor :type Actor%20Object%20Reference) (OtherComp :type Primitive%20Component%20Object%20Reference) (OtherBodyIndex :type Integer))
  ;[0.15 0.15 0.15 0.5] Display Inner/Outer icons
  (if (== (Game|GetPlayerCharacter 0) OtherActor)
    (Development|SetHiddeninGame (Variables|Default|GetInnerIcon) true false)
    (Development|SetHiddeninGame (Variables|Default|GetOuterIcon) false false)))

(event OnComponentBeginOverlap(OuterIconRadius)
  (params (OverlappedComponent :type Primitive%20Component%20Object%20Reference) (OtherActor :type Actor%20Object%20Reference) (OtherComp :type Primitive%20Component%20Object%20Reference) (OtherBodyIndex :type Integer) (bFromSweep :type Boolean) (SweepResult :type Hit%20Result%20Structure%20%28by%20ref%29))
  ;[0.15 0.15 0.15 0.5] Display Inner/Outer icons
  (if (== OtherActor (Game|GetPlayerCharacter 0))
    (Development|SetHiddeninGame (Variables|Default|GetOuterIcon) false false)))

(event OnComponentEndOverlap(OuterIconRadius)
  (params (OverlappedComponent :type Primitive%20Component%20Object%20Reference) (OtherActor :type Actor%20Object%20Reference) (OtherComp :type Primitive%20Component%20Object%20Reference) (OtherBodyIndex :type Integer))
  ;[0.15 0.15 0.15 0.5] Display Inner/Outer icons
  (if (== (Game|GetPlayerCharacter 0) OtherActor)
    (Development|SetHiddeninGame (Variables|Default|GetOuterIcon) true false)))

(event Custom|OpenCloseDoor
  ;[0.15 0.15 0.15 0.5] Open/Close door
  (Utilities|FlowControl|FlipFlop
    (:A
      (bind _alpha (Timeline|Door_TL Play)
        (:Update
          (Transformation|SetRelativeRotation (Variables|Default|GetDoor) (Math|Rotator|MakeRotator 0.0 0.0 (Math|Float|Lerp 0.0 -85.0 _alpha)) false false)
          ;[0.15 0.15 0.15 0.5] Move the inner/outer icons
          (Transformation|SetRelativeLocation (Variables|Default|GetInnerIcon) (Math|Vector|MakeVector 0.0 (Math|Float|Lerp -2e+01 0.0 _alpha) 5e+01) false false)
          (Transformation|SetRelativeLocation (Variables|Default|GetInnerIconOpposite) (Math|Vector|MakeVector 0.0 (Math|Float|Lerp 2e+01 0.0 _alpha) 5e+01) false false))))
    (:B
      (Timeline|Door_TL Reverse))))

(event EventBeginPlay
  ;[0.15 0.15 0.15 0.5] Create player reference
  (bind _asbp_third_person_character (Utilities|Casting|CastToBP_ThirdPersonCharacter (Game|GetPlayerCharacter 0)))
  (Variables|Default|SetPlayerRef _asbp_third_person_character)
  (Default|DialogueRowNum (Variables|Default|GetBP_DialogueComponent) "3"))

(event EventTrigger
  (params (TriggerNum :type Integer))
  ;[0.15 0.15 0.15 0.5] Trigger Switch for dialogue door. Trigger 1 goes to BP_LoneFire.
  (switch int TriggerNum
    (:2
      (bind _returnvalue (Actor|GetActorOfClass "/Game/VFX/Blueprints/LoneFire.LoneFire_C"))
      (Class|BPIInteraction|Trigger(Message) _returnvalue 2)
      (Default|LeaveDialogue (Variables|Default|GetBP_DialogueComponent self))
      (CallFunction|OpenCloseDoor))))

(event EventInteraction
  (params (playerRef :type BP%20Third%20Person%20Character%20Object%20Reference))
  ;[0.15 0.15 0.15 0.5] Open/Close door
)

(fn ConstructionScript
  ;[0.15 0.15 0.15 0.5] Set Icon Size
  (Transformation|SetWorldScale3D (Variables|Default|GetInnerIcon) (Math|Conversions|ToVector(Float) (/ (Variables|Default|GetIconSize) 1e+01)))
  ;[0.15 0.15 0.15 0.5] Set front Icon Location
  (Transformation|SetRelativeLocation (Variables|Default|GetOuterIcon) (Variables|Default|GetIconLocation) false false)
  ;[0.15 0.15 0.15 0.5] Set Icon location for opposite side
  (Transformation|SetRelativeLocation (Variables|Default|GetInnerIconOpposite) (Variables|Default|GetItemLocationBack) false false))