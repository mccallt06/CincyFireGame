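; Interactable dialogue window that passes player interactions to its dialogue component, with inner and outer icons shown by proximity overlaps.
; Numbered Trigger events swap its data table based on door state and sheet-dialogue progress, and relay triggers to the standing NPC, bed, sheet and player.
; OpenCloseDoor plays a sound and flip-flops a timeline that swings the Door and slides both sides' icons.
; The construction script sizes and positions the icons.
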(event OnComponentBeginOverlap(InnerIconRadius)
  (params (OverlappedComponent :type Primitive%20Component%20Object%20Reference) (OtherActor :type Actor%20Object%20Reference) (OtherComp :type Primitive%20Component%20Object%20Reference) (OtherBodyIndex :type Integer) (bFromSweep :type Boolean) (SweepResult :type Hit%20Result%20Structure%20%28by%20ref%29))
  ;[0.15 0.15 0.15 0.5] Display Inner/Outer icons
  (if (== OtherActor (Game|GetPlayerCharacter 0))
    (Development|SetHiddeninGame (Variables|Default|GetInnerIcon) false false)
    (Development|SetHiddeninGame (Variables|Default|GetOuterIcon) true false)))

(event OnComponentEndOverlap(InnerIconRadius)
  (params (OverlappedComponent :type Primitive%20Component%20Object%20Reference) (OtherActor :type Actor%20Object%20Reference) (OtherComp :type Primitive%20Component%20Object%20Reference) (OtherBodyIndex :type Integer))
  ;[0.15 0.15 0.15 0.5] Display Inner/Outer icons
  (if (== (Game|GetPlayerCharacter 0) OtherActor)
    (Development|SetHiddeninGame (Variables|Default|GetInnerIcon) true false)
    (Development|SetHiddeninGame (Variables|Default|GetOuterIcon) false false)))

(event OnComponentBeginOverlap(OuterIconRadius)
  (params (OverlappedComponent :type Primitive%20Component%20Object%20Reference) (OtherActor :type Actor%20Object%20Reference) (OtherComp :type Primitive%20Component%20Object%20Reference) (OtherBodyIndex :type Integer) (bFromSweep :type Boolean) (SweepResult :type Hit%20Result%20Structure%20%28by%20ref%29))
  ;[0.15 0.15 0.15 0.5] Display Inner/Outer icons
  (if (== OtherActor (Game|GetPlayerCharacter 0))
    (Development|SetHiddeninGame (Variables|Default|GetOuterIcon) false false)))

(event OnComponentEndOverlap(OuterIconRadius)
  (params (OverlappedComponent :type Primitive%20Component%20Object%20Reference) (OtherActor :type Actor%20Object%20Reference) (OtherComp :type Primitive%20Component%20Object%20Reference) (OtherBodyIndex :type Integer))
  ;[0.15 0.15 0.15 0.5] Display Inner/Outer icons
  (if (== (Game|GetPlayerCharacter 0) OtherActor)
    (Development|SetHiddeninGame (Variables|Default|GetOuterIcon) true false)))

(event Custom|OpenCloseDoor
  ;[0.15 0.15 0.15 0.5] Open/Close door
  (Audio|PlaySoundatLocation "/Game/Audio/SFX/SFX/SFX_OpenCloseDoor.SFX_OpenCloseDoor" (Transformation|GetActorLocation (Game|GetPlayerCharacter 0)) "0, 0, 0" 1.0 1.0 0.0 0 0 0 0)
  (Utilities|FlowControl|FlipFlop
    (:A
      (bind _alpha (Timeline|Door_TL Play)
        (:Update
          (Transformation|SetRelativeRotation (Variables|Default|GetDoor) (Math|Rotator|MakeRotator 0.0 0.0 (Math|Float|Lerp 0.0 -85.0 _alpha)) false false)
          ;[0.15 0.15 0.15 0.5] Move the inner/outer icons
          (Transformation|SetRelativeLocation (Variables|Default|GetInnerIcon) (Math|Vector|MakeVector 0.0 (Math|Float|Lerp -2e+01 0.0 _alpha) 5e+01) false false)
          (Transformation|SetRelativeLocation (Variables|Default|GetInnerIconOpposite) (Math|Vector|MakeVector 0.0 (Math|Float|Lerp 2e+01 0.0 _alpha) 5e+01) false false))))
    (:B
      (Timeline|Door_TL Reverse))))

(event EventBeginPlay
  ;[0.15 0.15 0.15 0.5] Create player reference
  (bind _asbp_third_person_character (Utilities|Casting|CastToBP_ThirdPersonCharacter (Game|GetPlayerCharacter 0)))
  (Variables|Default|SetPlayerRef _asbp_third_person_character))

(event EventTrigger
  (params (TriggerNum :type Integer))
  ;[0.15 0.15 0.15 0.5] Trigger Switch for dialogue window. Trigger 3 switches the data table of the window, trigger 4 sends a trigger to the bed to tell it to switch data tables. 5 means the door is open and switches the data table for that, 6 means the door is closed and switches the data table accordingly
  (switch int TriggerNum
    (:1
      (bind _returnvalue (Actor|GetActorOfClass "/Game/Characters/NPC_Blueprints/BP_NPCStanding.BP_NPCStanding_C"))
      (Default|Trigger _returnvalue 6))
    (:3
      (Variables|/Game/Dialogue/BP_DialogueComponent.BP_DialogueComponent_C|SetData%20Table (Variables|Default|GetBP_DialogueComponent) "/Game/Dialogue/DataTables/DT_Pedestrian2.DT_Pedestrian2")
      (Variables|Default|SetSheetDialogueDone true))
    (:4
      (bind _returnvalue_2 (Actor|GetActorOfClass "/Game/Blueprints/InteractionActors/BP_DialogueBed.BP_DialogueBed_C"))
      (Default|Trigger _returnvalue_2 3))
    (:5
      (Variables|Default|SetDoorClosed false)
      (Variables|/Game/Dialogue/BP_DialogueComponent.BP_DialogueComponent_C|SetData%20Table (Variables|Default|GetBP_DialogueComponent) "/Game/Dialogue/DataTables/DT_WindowDoorOpen.DT_WindowDoorOpen"))
    (:6
      (Variables|Default|SetDoorClosed true)
      (if (Variables|Default|GetSheetDialogueDone)
        (Variables|/Game/Dialogue/BP_DialogueComponent.BP_DialogueComponent_C|SetData%20Table (Variables|Default|GetBP_DialogueComponent) "/Game/Dialogue/DataTables/DT_Pedestrian2.DT_Pedestrian2")
        (else
          (Variables|/Game/Dialogue/BP_DialogueComponent.BP_DialogueComponent_C|SetData%20Table (Variables|Default|GetBP_DialogueComponent) "/Game/Dialogue/DataTables/DT_Pedestrian.DT_Pedestrian"))))
    (:7
      (bind _returnvalue_3 (Actor|GetActorOfClass "/Game/Blueprints/BP_Sheet.BP_Sheet_C"))
      (Default|Trigger _returnvalue_3 3)
      (Class|BPITrigger|Trigger(Message) (Game|GetPlayerCharacter 0) 15))))

(event EventInteraction
  (params (playerRef :type BP%20Third%20Person%20Character%20Object%20Reference))
  ;[0.15 0.15 0.15 0.5] Open/Close door
  (Default|Interaction (Variables|Default|GetBP_DialogueComponent) (Variables|Default|GetPlayerRef)))

(fn ConstructionScript
  ;[0.15 0.15 0.15 0.5] Set Icon Size
  (Transformation|SetWorldScale3D (Variables|Default|GetInnerIcon) (Math|Conversions|ToVector(Float) (/ (Variables|Default|GetIconSize) 1e+01)))
  ;[0.15 0.15 0.15 0.5] Set front Icon Location
  (Transformation|SetRelativeLocation (Variables|Default|GetOuterIcon) (Variables|Default|GetIconLocation) false false)
  ;[0.15 0.15 0.15 0.5] Set Icon location for opposite side
  (Transformation|SetRelativeLocation (Variables|Default|GetInnerIconOpposite) (Variables|Default|GetItemLocationBack) false false))