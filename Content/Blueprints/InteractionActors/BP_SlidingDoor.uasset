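; Interactable sliding door actor that toggles open and closed each time its Interaction event fires.
; A FlipFlop plays or reverses a timeline that lerps the door's relative location along X, with a sound played at the player's location.
; Two overlap radii swap outer and inner prompt icons as the player approaches or leaves.
; The construction script applies configurable size and location to both icons.
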(event OnComponentBeginOverlap(InnerIconRadius)
  (params (OverlappedComponent :type Primitive%20Component%20Object%20Reference) (OtherActor :type Actor%20Object%20Reference) (OtherComp :type Primitive%20Component%20Object%20Reference) (OtherBodyIndex :type Integer) (bFromSweep :type Boolean) (SweepResult :type Hit%20Result%20Structure%20%28by%20ref%29))
  ;[0.15 0.15 0.15 0.5] Display inner/outer icons
  (if (== OtherActor (Game|GetPlayerCharacter 0))
    (Development|SetHiddeninGame (Variables|Default|GetInnerIcon) false false)
    (Development|SetHiddeninGame (Variables|Default|GetOuterIcon) true false)))

(event OnComponentEndOverlap(InnerIconRadius)
  (params (OverlappedComponent :type Primitive%20Component%20Object%20Reference) (OtherActor :type Actor%20Object%20Reference) (OtherComp :type Primitive%20Component%20Object%20Reference) (OtherBodyIndex :type Integer))
  ;[0.15 0.15 0.15 0.5] Display inner/outer icons
  (if (== (Game|GetPlayerCharacter 0) OtherActor)
    (Development|SetHiddeninGame (Variables|Default|GetInnerIcon) true false)
    (Development|SetHiddeninGame (Variables|Default|GetOuterIcon) false false)))

(event OnComponentBeginOverlap(OuterIconRadius)
  (params (OverlappedComponent :type Primitive%20Component%20Object%20Reference) (OtherActor :type Actor%20Object%20Reference) (OtherComp :type Primitive%20Component%20Object%20Reference) (OtherBodyIndex :type Integer) (bFromSweep :type Boolean) (SweepResult :type Hit%20Result%20Structure%20%28by%20ref%29))
  ;[0.15 0.15 0.15 0.5] Display inner/outer icons
  (if (== OtherActor (Game|GetPlayerCharacter 0))
    (Development|SetHiddeninGame (Variables|Default|GetOuterIcon) false false)))

(event OnComponentEndOverlap(OuterIconRadius)
  (params (OverlappedComponent :type Primitive%20Component%20Object%20Reference) (OtherActor :type Actor%20Object%20Reference) (OtherComp :type Primitive%20Component%20Object%20Reference) (OtherBodyIndex :type Integer))
  ;[0.15 0.15 0.15 0.5] Display inner/outer icons
  (if (== (Game|GetPlayerCharacter 0) OtherActor)
    (Development|SetHiddeninGame (Variables|Default|GetOuterIcon) true false)))

(event Custom|OpenCloseDoor
  ;[0.15 0.15 0.15 0.5] Open/Close door
  (Audio|PlaySoundatLocation "/Game/Audio/SFX/SFX/SFX_SlidingDoor.SFX_SlidingDoor" (Transformation|GetActorLocation (Game|GetPlayerCharacter 0)) "0, 0, 0" 1.0 1.0 0.0 0 "/Game/Audio/SFX_Conccurency.SFX_Conccurency" 0 0)
  (Utilities|FlowControl|FlipFlop
    (:A
      (bind _alpha (Timeline|Door_TL Play)
        (:Update
          (Transformation|SetRelativeLocation (Variables|Default|GetSliding_Door) (Math|Vector|Lerp(Vector) "0, 0, 0" "100.000000,0.000000,0.000000" _alpha) false false))))
    (:B
      (Timeline|Door_TL Reverse))))

(event EventBeginPlay
  ;[0.15 0.15 0.15 0.5] Create player reference
  (bind _asbp_third_person_character (Utilities|Casting|CastToBP_ThirdPersonCharacter (Game|GetPlayerCharacter 0)))
  (Variables|Default|SetPlayerRef _asbp_third_person_character))

(event EventInteraction
  (params (playerRef :type BP%20Third%20Person%20Character%20Object%20Reference))
  ;[0.15 0.15 0.15 0.5] Open/Close door
  (CallFunction|OpenCloseDoor))

(fn ConstructionScript
  ;[0.15 0.15 0.15 0.5] Set Icon Size
  (Transformation|SetWorldScale3D (Variables|Default|GetInnerIcon) (Math|Conversions|ToVector(Float) (/ (Variables|Default|GetIconSize) 1e+01)))
  ;[0.15 0.15 0.15 0.5] Set Icon Location
  (Transformation|SetRelativeLocation (Variables|Default|GetOuterIcon) (Variables|Default|GetIconLocation) false false))