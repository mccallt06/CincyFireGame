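; Interactable bed that runs dialogue through BPDialogueComponent and shows near or far prompt icons from two overlap radii, sized and placed in the construction script.
; Numbered triggers play a scripted hide sequence, swap the dialogue table to DT_Bed2, or forward to BP_DialogueWindow.
; The hide sequence disables input, fades out, forces prone, relocates the player mesh, fades in, then restarts dialogue, which stays locked meanwhile.
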(event OnComponentBeginOverlap(InnerIconRadius)
  (params (OverlappedComponent :type Primitive%20Component%20Object%20Reference) (OtherActor :type Actor%20Object%20Reference) (OtherComp :type Primitive%20Component%20Object%20Reference) (OtherBodyIndex :type Integer) (bFromSweep :type Boolean) (SweepResult :type Hit%20Result%20Structure%20%28by%20ref%29))
  ;[0.15 0.15 0.15 0.5] Display Inner/Outer icons
  (if (== OtherActor (Game|GetPlayerCharacter 0))
    (Development|SetHiddeninGame (Variables|Default|GetInnerIcon) false false)
    (Development|SetHiddeninGame (Variables|Default|GetOuterIcon) true false)))

(event OnComponentEndOverlap(InnerIconRadius)
  (params (OverlappedComponent :type Primitive%20Component%20Object%20Reference) (OtherActor :type Actor%20Object%20Reference) (OtherComp :type Primitive%20Component%20Object%20Reference) (OtherBodyIndex :type Integer))
  ;[0.15 0.15 0.15 0.5] Display Inner/Outer icons
  (if (== (Game|GetPlayerCharacter 0) OtherActor)
    (Development|SetHiddeninGame (Variables|Default|GetInnerIcon) true false)
    (Development|SetHiddeninGame (Variables|Default|GetOuterIcon) false false)))

(event OnComponentBeginOverlap(OuterIconRadius)
  (params (OverlappedComponent :type Primitive%20Component%20Object%20Reference) (OtherActor :type Actor%20Object%20Reference) (OtherComp :type Primitive%20Component%20Object%20Reference) (OtherBodyIndex :type Integer) (bFromSweep :type Boolean) (SweepResult :type Hit%20Result%20Structure%20%28by%20ref%29))
  ;[0.15 0.15 0.15 0.5] Display Inner/Outer icons
  (if (== OtherActor (Game|GetPlayerCharacter 0))
    (Development|SetHiddeninGame (Variables|Default|GetOuterIcon) false false)))

(event OnComponentEndOverlap(OuterIconRadius)
  (params (OverlappedComponent :type Primitive%20Component%20Object%20Reference) (OtherActor :type Actor%20Object%20Reference) (OtherComp :type Primitive%20Component%20Object%20Reference) (OtherBodyIndex :type Integer))
  ;[0.15 0.15 0.15 0.5] Display Inner/Outer icons
  (if (== (Game|GetPlayerCharacter 0) OtherActor)
    (Development|SetHiddeninGame (Variables|Default|GetOuterIcon) true false)))

(event EventBeginPlay
  ;[0.15 0.15 0.15 0.5] Create player reference
  (bind _asbp_third_person_character (Utilities|Casting|CastToBP_ThirdPersonCharacter (Game|GetPlayerCharacter 0)))
  (Variables|Default|SetPlayerRef _asbp_third_person_character))

(event EventTrigger
  (params (TriggerNum :type Integer))
  (bind _returnvalue (Game|GetPlayerCharacter 0))
  (bind _returnvalue_2 (Game|GetPlayerCharacter 0))
  (bind _returnvalue_3 (Game|GetPlayerController 0))
  (bind _returnvalue_4 (Game|GetPlayerCameraManager 0))
  ;[0.15 0.15 0.15 0.5] Trigger switch for dialogue blueprint
  (switch int TriggerNum
    (:2
      ;[0.15 0 0.001944 0.5] Bed hide sequence
      (Class|BPITrigger|Trigger(Message) _returnvalue_2 11)
      (Class|BPITrigger|Trigger(Message) _returnvalue_2 16)
      (Input|SetIgnoreMoveInput _returnvalue_3 true)
      (Input|SetIgnoreLookInput _returnvalue_3 true)
      (CameraFades|StartCameraFade :self _returnvalue_4 :ToAlpha 1.0 :Duration 3.0 :bHoldWhenFinished true)
      (bind _asbp_third_person_character (Utilities|Casting|CastToBP_ThirdPersonCharacter _returnvalue))
      (Variables|Default|SetDialogueLock true)
      (Default|ForceProneToggle _asbp_third_person_character)
      (Utilities|FlowControl|Delay 3.0)
      (Transformation|SetWorldLocation (Variables|/Script/Engine.Character|GetMesh _returnvalue) "-2220.000000,670.000000,280.000000" false false)
      (Utilities|FlowControl|Delay 2.0)
      (CameraFades|StartCameraFade :self _returnvalue_4 :FromAlpha 1.0 :Duration 3.0 :bHoldWhenFinished true)
      (bind _outactors (Actor|GetAllActorsOfClass "/Game/UI/ItemText/BP_TriggerBased.BP_TriggerBased_C"))
      (Class|BPIInteraction|Trigger(Message) (Utilities|Array|Get(acopy) _outactors) 3)
      (Variables|Default|SetDialogueLock false)
      (CallFunction|Interaction)
      (Utilities|FlowControl|DelayUntilNextTick)
      (bind _asbp_third_person_character_2 (Utilities|Casting|CastToBP_ThirdPersonCharacter (Game|GetPlayerCharacter 0)))
      (Variables|/Game/ThirdPerson/Blueprints/BP_ThirdPersonCharacter.BP_ThirdPersonCharacter_C|SetInText _asbp_third_person_character_2 true))
    (:3
      (Variables|/Game/Dialogue/BP_DialogueComponent.BP_DialogueComponent_C|SetData%20Table (Variables|Default|GetBP_DialogueComponent) "/Game/Dialogue/DataTables/DT_Bed2.DT_Bed2"))
    (:4
      (bind _returnvalue_5 (Actor|GetActorOfClass "/Game/Blueprints/InteractionActors/BP_DialogueWindow.BP_DialogueWindow_C"))
      (Default|Trigger _returnvalue_5 3))))

(event EventInteraction
  (params (playerRef :type BP%20Third%20Person%20Character%20Object%20Reference))
  (if (not (Variables|Default|GetDialogueLock))
    (Default|Interaction (Variables|Default|GetBP_DialogueComponent) (Variables|Default|GetPlayerRef))))

(fn ConstructionScript
  ;[0.15 0.15 0.15 0.5] Set Icon Size
  (Transformation|SetWorldScale3D (Variables|Default|GetInnerIcon) (Math|Conversions|ToVector(Float) (/ (Variables|Default|GetIconSize) 1e+01)))
  ;[0.15 0.15 0.15 0.5] Set front Icon Location
  (Transformation|SetRelativeLocation (Variables|Default|GetOuterIcon) (Variables|Default|GetIconLocation) false false))